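; Animal character Blueprint that computes ground-adaptive IK for four limbs, two hands and two feet.
; When IK is enabled, BeginPlay and Tick run FootPlacement and enable foot position and rotation alphas only while walking.
; TraceIKEffector line-traces along the capsule's up axis, shifting the start back by ForwardSpeed, and derives mesh-space height and slope rotation.
; Grounded limbs interpolate toward these results; ungrounded limbs keep their last values.
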(event `self.ReceiveBeginPlay`
  (bind _returnvalue (`KismetMathLibrary.SelectFloat` 1.0 0.0 (`CharacterMovementComponent.IsWalking` (`self.CharacterMovement`))))
  ;[1 1 1] Whether to use IK.
  (if (`self.IsIK`) :!label _label
    (`self.FootPlacement`)
    (set `self.IKAlpha` 1.0)
    (set `self.IKFootPosAlpha` _returnvalue)
    (set `self.IKFootRotAlpha` _returnvalue)
    (else
      (set `self.IKAlpha` 0.0))))

(event `self.ReceiveTick`
  (params (DeltaSeconds :type "Float (single-precision)"))
  (set `self.DeltaTime` DeltaSeconds)
  (goto _label))

(fn `FootPlacement`
  ;[1 1 1] L_Hand
  (bind (_footisgrounded _footrot _ikposoffset) (`self.Trace IKEffector` (`self.L_HandName`) (`self.Trace Distance`)))
  (if _footisgrounded
    (set `self.L_HandIKOffset` (`KismetMathLibrary.VInterpTo` (`self.L_HandIKOffset`) _ikposoffset (`self.DeltaTime`) (`self.IKInterpSpeed`)))
    (set `self.L_HandRot` (`KismetMathLibrary.RInterpTo` (`self.L_HandRot`) _footrot (`self.DeltaTime`) (`self.IKInterpSpeed`))))
  ;[1 1 1] R_Hand
  (bind (_footisgrounded_2 _footrot_2 _ikposoffset_2) (`self.Trace IKEffector` (`self.R_HandName`) (`self.Trace Distance`)))
  (if _footisgrounded_2
    (set `self.R_HandIKOffset` (`KismetMathLibrary.VInterpTo` (`self.R_HandIKOffset`) _ikposoffset_2 (`self.DeltaTime`) (`self.IKInterpSpeed`)))
    (set `self.R_HandRot` (`KismetMathLibrary.RInterpTo` (`self.R_HandRot`) _footrot_2 (`self.DeltaTime`) (`self.IKInterpSpeed`))))
  ;[1 1 1] L_Foot
  (bind (_footisgrounded_3 _footrot_3 _ikposoffset_3) (`self.Trace IKEffector` (`self.L_FootName`) (`self.Trace Distance`)))
  (if _footisgrounded_3
    (set `self.L_FootIKOffset` (`KismetMathLibrary.VInterpTo` (`self.L_FootIKOffset`) _ikposoffset_3 (`self.DeltaTime`) (`self.IKInterpSpeed`)))
    (set `self.L_FootRot` (`KismetMathLibrary.RInterpTo` (`self.L_FootRot`) _footrot_3 (`self.DeltaTime`) (`self.IKInterpSpeed`))))
  ;[1 1 1] R_Foot
  (bind (_footisgrounded_4 _footrot_4 _ikposoffset_4) (`self.Trace IKEffector` (`self.R_FootName`) (`self.Trace Distance`)))
  (if _footisgrounded_4
    (set `self.R_FootIKOffset` (`KismetMathLibrary.VInterpTo` (`self.R_FootIKOffset`) _ikposoffset_4 (`self.DeltaTime`) (`self.IKInterpSpeed`)))
    (set `self.R_FootRot` (`KismetMathLibrary.RInterpTo` (`self.R_FootRot`) _footrot_4 (`self.DeltaTime`) (`self.IKInterpSpeed`)))))

(fn `Trace IKEffector`
  (params (FootName :type Name) (TraceDistance :type "Float (double-precision)") (HeightOffset :type "Float (double-precision)"))
  (returns (FootIsGrounded :type Boolean) (FootRot :type "Rotator Structure") (IKPosOffset :type "Vector Structure"))
  (bind _mesh (`self.Mesh`))
  (bind _returnvalue (`SceneComponent.GetSocketLocation` (`self.Mesh`) FootName))
  (bind _returnvalue_2 (* (`SceneComponent.GetUpVector` (`self.CapsuleComponent`)) TraceDistance))
  ;[1 1 1] Trace from foot.
  (bind (_outhit _returnvalue_3) (`KismetSystemLibrary.LineTraceSingle` (+ _returnvalue (+ _returnvalue_2 (* (`SceneComponent.GetForwardVector` (`self.CapsuleComponent`)) (* (`self.ForwardSpeed`) -1.0)))) (- _returnvalue _returnvalue_2) "TraceTypeQuery1" true))
  (if _returnvalue_3
    (bind (_bblockinghit _binitialoverlap _time _distance _location _impactpoint _normal) (`GameplayStatics.BreakHitResult` _outhit))
    (bind _returnvalue_4 (`KismetMathLibrary.Cross_VectorVector` (`SceneComponent.GetUpVector` _mesh) (`KismetMathLibrary.InverseTransformDirection` (`SceneComponent.K2_GetComponentToWorld` _mesh) _normal)))
    ;[1 1 1] Calculate IKHeightOffset in Meshe's coordinate.
    (return _returnvalue_3 (`KismetMathLibrary.SelectRotator` (`KismetMathLibrary.RotatorFromAxisAndAngle` _returnvalue_4 (`KismetMathLibrary.DegAsin` (`KismetMathLibrary.VSize` _returnvalue_4))) (struct) _returnvalue_3) (`KismetMathLibrary.MakeVector` 0.0 0.0 (- (.z (`KismetMathLibrary.InverseTransformLocation` (`SceneComponent.K2_GetComponentToWorld` (`self.Mesh`)) _location)) HeightOffset)))
    (else
      (return false (struct) (`KismetMathLibrary.MakeVector` 0.0 0.0 (`self.MaxLegIKOffset`))))))

(fn `UserConstructionScript`)